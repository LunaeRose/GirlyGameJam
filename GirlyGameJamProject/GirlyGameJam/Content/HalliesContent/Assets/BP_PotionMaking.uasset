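; BP_PotionMaking is a potion-making station where the player sets down and picks up the carried cauldron.
; On BeginPlay it finds the BP_Cauldron actor, and on overlap it caches the first-person character.
; StartInteract toggles the cauldron by attachment, snapping it to the station's SMCauldron or reattaching it to the character's Cube with world transform kept.
; IsSetDown and the cauldron's IsCarrying flag track the state according to each attach result.
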(event EventBeginPlay
  (bind _returnvalue (Actor|GetActorOfClass "/Game/HalliesContent/Assets/BP_Cauldron.BP_Cauldron_C"))
  (Variables|Default|SetCarriedCauldron _returnvalue)
  (Variables|Default|SetIsSetDown? false))

(event Collision|EventActorBeginOverlap
  (params (OtherActor :type Actor%20Object%20Reference))
  (bind _asbp_first_person_character (Utilities|Casting|CastToBP_FirstPersonCharacter OtherActor))
  (Variables|Default|SetAs%20BP%20First%20Person%20Character _asbp_first_person_character))

(event EventTick
  (params (DeltaSeconds :type Float%20%28single-precision%29)))

(event EventStartInteract
  (params (InteractingActor :type Actor%20Object%20Reference))
  (bind _carriedcauldron (Variables|Default|GetCarriedCauldron))
  (if (Variables|/Game/HalliesContent/Assets/BP_Cauldron.BP_Cauldron_C|GetIsCarrying? _carriedcauldron)
    (bind _returnvalue (Transformation|AttachComponentToComponent _carriedcauldron (Variables|Default|GetSM_Cauldron) "None" "SnapToTarget" "SnapToTarget" "SnapToTarget" true))
    (if _returnvalue
      (Variables|Default|SetIsSetDown? true)
      (Variables|/Game/HalliesContent/Assets/BP_Cauldron.BP_Cauldron_C|SetIsCarrying? (Variables|Default|GetCarriedCauldron) false)
      (else
        (Variables|Default|SetIsSetDown? false)
        (Variables|/Game/HalliesContent/Assets/BP_Cauldron.BP_Cauldron_C|SetIsCarrying? (Variables|Default|GetCarriedCauldron) true)))
    (elif (Variables|Default|GetIsSetDown?)
      (bind _returnvalue_2 (Transformation|AttachComponentToComponent (Variables|Default|GetCarriedCauldron) (Variables|/Game/FirstPerson/Blueprints/BP_FirstPersonCharacter.BP_FirstPersonCharacter_C|GetCube (Variables|Default|GetAs%20BP%20First%20Person%20Character)) "None" "KeepWorld" "KeepWorld" "KeepWorld" true))
      (if _returnvalue_2
        (Variables|Default|SetIsSetDown? false)
        (Variables|/Game/HalliesContent/Assets/BP_Cauldron.BP_Cauldron_C|SetIsCarrying? (Variables|Default|GetCarriedCauldron) true)
        (else
          (Variables|Default|SetIsSetDown? true)
          (Variables|/Game/HalliesContent/Assets/BP_Cauldron.BP_Cauldron_C|SetIsCarrying? (Variables|Default|GetCarriedCauldron) false)))
      (else
        (Development|PrintString "Nothing to pick up!" true true "(R=1.000000,G=0.000000,B=0.022786,A=1.000000)" 5.0)))))

(fn ConstructionScript)