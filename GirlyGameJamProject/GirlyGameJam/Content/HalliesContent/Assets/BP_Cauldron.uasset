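; BP_Cauldron is a cauldron actor the first-person player can pick up and drop, limited to one carried item at a time.
; StartInteract checks HandsFull, then registers itself as CarriedItem, disables physics and collision, attaches to the character's Cube, snaps there after a short delay and hides the interact prompt.
; DropItem only restores physics and collision; the explicit detach sits in unconnected nodes.
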(event EventBeginPlay
  (bind _returnvalue (Actor|GetActorOfClass "/Game/FirstPerson/Blueprints/BP_FirstPersonCharacter.BP_FirstPersonCharacter_C"))
  (Variables|Default|SetPlayerCharacter _returnvalue)
  (Variables|Default|SetIsCarrying? false)
  (Collision|SetActorEnableCollision true))

(event Collision|EventActorBeginOverlap
  (params (OtherActor :type Actor%20Object%20Reference)))

(event EventTick
  (params (DeltaSeconds :type Float%20%28single-precision%29)))

(event EventStartInteract
  (params (InteractingActor :type Actor%20Object%20Reference))
  (bind _playercharacter (Variables|Default|GetPlayerCharacter))
  (bind _playercharacter_2 (Variables|Default|GetPlayerCharacter))
  (bind _cube (Variables|/Game/FirstPerson/Blueprints/BP_FirstPersonCharacter.BP_FirstPersonCharacter_C|GetCube _playercharacter_2))
  (bind _returnvalue (Transformation|GetWorldTransform _cube))
  (if (Variables|/Game/FirstPerson/Blueprints/BP_FirstPersonCharacter.BP_FirstPersonCharacter_C|GetHandsFull _playercharacter)
    (Development|PrintString "Can't Carry more than 1 thing!!!" true true "(R=1.000000,G=0.010319,B=0.023582,A=1.000000)" 5.0)
    (else
      (Variables|/Game/FirstPerson/Blueprints/BP_FirstPersonCharacter.BP_FirstPersonCharacter_C|SetCarriedItem _playercharacter self)
      (Variables|/Game/FirstPerson/Blueprints/BP_FirstPersonCharacter.BP_FirstPersonCharacter_C|SetHandsFull _playercharacter true)
      (Physics|SetSimulatePhysics (Variables|Default|GetSM_Cauldron) false)
      (bind _returnvalue_2 (Transformation|AttachComponentToComponent _cube "None" "KeepWorld" "KeepWorld" "KeepWorld" false))
      (Utilities|FlowControl|Delay 0.1)
      (Transformation|SetActorTransform (Math|Transform|MakeTransform (.location _returnvalue) (.rotation _returnvalue) "1.000000,1.000000,1.000000"))
      (Variables|Default|SetIsCarrying? true)
      (Collision|SetActorEnableCollision false)
      (Variables|/Script/UMG.Widget|SetVisibility (Variables|/Game/HalliesContent/Menu/UI_Interact.UI_Interact_C|GetEtoInteract (Variables|/Game/FirstPerson/Blueprints/BP_FirstPersonCharacter.BP_FirstPersonCharacter_C|GetUIInteract (Variables|Default|GetPlayerCharacter))) "Hidden"))))

(event EventDropItem
  (Physics|SetSimulatePhysics (Variables|Default|GetSM_Cauldron) true)
  (Collision|SetActorEnableCollision true))

(fn ConstructionScript)