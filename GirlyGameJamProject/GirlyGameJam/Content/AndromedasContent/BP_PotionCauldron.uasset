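; BP_PotionCauldron is an interactable cauldron that checks the player's inventory against a potion recipe.
; On BeginPlay it caches the first-person player character to reach that character's inventory component.
; StartInteract compares the whole inventory to its Recipe array with an Array Identical check.
; Either result clears the inventory and only prints whether the recipe was correct, with no potion produced.
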(event EventBeginPlay
  ;[1 1 1] player reference
  (bind _asbp_first_person_character (Utilities|Casting|CastToBP_FirstPersonCharacter (Game|Player|GetPlayerPawn 0)))
  (Variables|Default|SetAs%20BP%20First%20Person%20Character _asbp_first_person_character))

(event EventStartInteract
  (params (InteractingActor :type Actor%20Object%20Reference))
  (bind _as_bp_first_person_character (Variables|Default|GetAs%20BP%20First%20Person%20Character))
  (bind _bpc_inventory (Variables|/Game/FirstPerson/Blueprints/BP_FirstPersonCharacter.BP_FirstPersonCharacter_C|GetBPC_Inventory _as_bp_first_person_character))
  (if (Utilities|Array|Identical (Variables|/Game/AndromedasContent/BPC_Inventory.BPC_Inventory_C|GetInventory _bpc_inventory) (Variables|Default|GetRecipe))
    (Default|ClearInventory _bpc_inventory)
    (Development|PrintString "correct recipe!")
    (else
      (Default|ClearInventory _bpc_inventory)
      (Development|PrintString "incorrect recipe!"))))

(fn ConstructionScript)