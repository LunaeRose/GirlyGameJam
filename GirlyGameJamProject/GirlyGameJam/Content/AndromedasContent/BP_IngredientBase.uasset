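; Base actor for ingredient pickups that the player collects into their inventory by interacting with them.
; The construction script applies the configurable StaticMesh to the Ingredient component.
; BeginPlay caches a reference to the first-person player character.
; StartInteract adds ItemName to that character's BPCInventory component, then destroys the actor.
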(event EventBeginPlay
  ;[1 1 1] Reference Player
  (bind _asbp_first_person_character (Utilities|Casting|CastToBP_FirstPersonCharacter (Game|Player|GetPlayerPawn 0)))
  (Variables|Default|SetAs%20BP%20First%20Person%20Character _asbp_first_person_character))

(event EventStartInteract
  (params (InteractingActor :type Actor%20Object%20Reference))
  ;[1 1 1] Pick up item, add it to Inventory by item name, destroy actor
  (Default|AddItemtoInventory (Variables|/Game/FirstPerson/Blueprints/BP_FirstPersonCharacter.BP_FirstPersonCharacter_C|GetBPC_Inventory (Variables|Default|GetAs%20BP%20First%20Person%20Character)) (Variables|Default|GetItemName))
  (Actor|DestroyActor))

(fn ConstructionScript
  (Components|StaticMesh|SetStaticMesh (Variables|Default|GetIngredient) (Variables|Default|GetStaticMesh)))