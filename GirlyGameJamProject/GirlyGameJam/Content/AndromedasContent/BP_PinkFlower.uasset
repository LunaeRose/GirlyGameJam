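; BP_PinkFlower is an interactable pink flower pickup that respawns after being taken.
; On BeginPlay it caches the BP_FirstPersonCharacter found in the level.
; StartInteract passes the flower to that character's AddItemMessage, then hides it and disables collision after a brief delay.
; The same actor is reused rather than destroyed, becoming visible and collidable again two minutes later.
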(event EventBeginPlay
  (bind _returnvalue (Actor|GetActorOfClass "/Game/FirstPerson/Blueprints/BP_FirstPersonCharacter.BP_FirstPersonCharacter_C"))
  (Variables|Default|SetCharacter _returnvalue))

(event EventStartInteract
  (params (InteractingActor :type Actor%20Object%20Reference))
  (Class|BPIInventory|AddItem(Message) (Variables|Default|GetCharacter) self)
  (Utilities|FlowControl|Delay 0.2)
  (Rendering|SetActorHiddenInGame true)
  (Collision|SetActorEnableCollision false)
  (Utilities|FlowControl|Delay 1.2e+02)
  (Rendering|SetActorHiddenInGame false)
  (Collision|SetActorEnableCollision true))

(fn ConstructionScript)