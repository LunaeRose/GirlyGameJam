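; BP_Potion_Base is a carryable potion that the first-person player picks up and drops.
; StartInteract refuses when the player's hands are full; otherwise it registers as CarriedItem, disables physics and attaches to the player's Cube.
; After a short delay it snaps to the Cube and hides the interact prompt.
; DropItem only re-enables physics; a note reports that re-picked potions fail to follow the player.
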(event EventDropItem
  ;[1 0.3294 0] This is largely the same as the cauldron, but with the changes that I think are better for tracking the carried item. I also think the branch after attaching was unnecessary, as this functions without it. Still troubleshooting picking potions up multiple times. The only issue is that the potion doesn't actually follow the player again after dropping it once.
  (Physics|SetSimulatePhysics (Variables|Default|GetCylinder) true))

(event EventStartInteract
  (params (InteractingActor :type Actor%20Object%20Reference))
  (bind _player (Variables|Default|GetPlayer))
  (bind _player_2 (Variables|Default|GetPlayer))
  (bind _cube (Variables|/Game/FirstPerson/Blueprints/BP_FirstPersonCharacter.BP_FirstPersonCharacter_C|GetCube _player_2))
  (bind _returnvalue (Transformation|GetWorldTransform _cube))
  ;[1 0.3294 0] This is largely the same as the cauldron, but with the changes that I think are better for tracking the carried item. I also think the branch after attaching was unnecessary, as this functions without it. Still troubleshooting picking potions up multiple times. The only issue is that the potion doesn't actually follow the player again after dropping it once.
  (if (Variables|/Game/FirstPerson/Blueprints/BP_FirstPersonCharacter.BP_FirstPersonCharacter_C|GetHandsFull (Variables|Default|GetPlayer))
    (Development|PrintString "Can't Carry more than 1 thing!!!" true true "(R=1.000000,G=0.010319,B=0.023582,A=1.000000)" 5.0)
    (else
      (Variables|/Game/FirstPerson/Blueprints/BP_FirstPersonCharacter.BP_FirstPersonCharacter_C|SetCarriedItem _player self)
      (Variables|/Game/FirstPerson/Blueprints/BP_FirstPersonCharacter.BP_FirstPersonCharacter_C|SetHandsFull _player true)
      (Physics|SetSimulatePhysics (Variables|Default|GetCylinder) false)
      (Transformation|AttachComponentToComponent _cube "None" "KeepWorld" "KeepWorld" "KeepWorld" false)
      (Utilities|FlowControl|Delay 0.1)
      (Transformation|SetActorTransform (Math|Transform|MakeTransform (.location _returnvalue) (.rotation _returnvalue) "1.000000,1.000000,1.000000"))
      (Variables|/Script/UMG.Widget|SetVisibility (Variables|/Game/HalliesContent/Menu/UI_Interact.UI_Interact_C|GetEtoInteract (Variables|/Game/FirstPerson/Blueprints/BP_FirstPersonCharacter.BP_FirstPersonCharacter_C|GetUIInteract (Variables|Default|GetPlayer))) "Hidden"))))

(event EventBeginPlay
  ;[1 0.3294 0] This is largely the same as the cauldron, but with the changes that I think are better for tracking the carried item. I also think the branch after attaching was unnecessary, as this functions without it. Still troubleshooting picking potions up multiple times. The only issue is that the potion doesn't actually follow the player again after dropping it once.
  (bind _asbp_first_person_character (Utilities|Casting|CastToBP_FirstPersonCharacter (Game|Player|GetPlayerPawn 0)))
  (Variables|Default|SetPlayer _asbp_first_person_character))

(fn ConstructionScript)